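; Breakout-style block that loses a life each time bp_ball hits it and is destroyed when none remain.
; The construction script rolls a random starting life, which sets the cube's metal material and its point value.
; Each hit swaps the material to match the remaining life; at zero it fires the BlockDestroyed dispatcher with its value before destroying itself.
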(event `self.ReceiveHit`
  (params (MyComp :type "PrimitiveComponent Object Reference") (Other :type "Actor Object Reference") (OtherComp :type "PrimitiveComponent Object Reference") (bSelfMoved :type Boolean) (HitLocation :type "Vector Structure") (HitNormal :type "Vector Structure") (NormalImpulse :type "Vector Structure") (Hit :type "HitResult Structure (by ref)"))
  (cast `/Game/mystuff/blueprints/bp_ball` Other)
  (`self.ballhit`))

(event `ballhit`
  (bind _cube (`self.Cube`))
  ;[1 1 1] менять цвет при ударе, сломать если жизней у объекта меньше нуля
  (bind _result (`/Engine/EditorBlueprintResources/StandardMacros.DecrementInt` (`self.life`))
    (:`  `
      (switch `int` _result
        (:`0`
          ;[1 1 1] dispatch event для уничтоженного блока, скидывает очки за него
          (`self.BlockDestroyed` (`self.value`))
          (`self.K2_DestroyActor`))
        (:`1`
          (`PrimitiveComponent.SetMaterial` _cube 0 "/Game/mystuff/materials/metal/mt_metal_base.mt_metal_base"))
        (:`2`
          (`PrimitiveComponent.SetMaterial` _cube 0 "/Game/mystuff/materials/metal/mt_metal_iron.mt_metal_iron"))))))

(fn `UserConstructionScript`
  (bind _cube (`self.Cube`))
  ;[1 1 1] создать рандомное количество жизней у объекта
  (bind _output_get (set `self.life` (`KismetMathLibrary.RandomIntegerInRange` 1 3)))
  ;[1 1 1] меняем цвет в зависимости от количества жизней у блоков
  (switch `int` _output_get
    (:`1`
      (`PrimitiveComponent.SetMaterial` _cube 0 "/Game/mystuff/materials/metal/mt_metal_base.mt_metal_base")
      (set `self.value` 100))
    (:`2`
      (`PrimitiveComponent.SetMaterial` _cube 0 "/Game/mystuff/materials/metal/mt_metal_iron.mt_metal_iron")
      (set `self.value` 150))
    (:`3`
      (`PrimitiveComponent.SetMaterial` _cube 0 "/Game/mystuff/materials/metal/mt_metal_gold.mt_metal_gold")
      (set `self.value` 200))))