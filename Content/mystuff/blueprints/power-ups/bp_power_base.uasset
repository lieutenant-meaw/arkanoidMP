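; Base power-up actor that travels across the level with a randomly chosen power type, shown as a text label.
; Each tick it moves in X and Y by speed and direction, with collision sweep.
; The construction script randomizes the Power enum, writes its name to the TextRender, and sets the cone to blue, green or red.
; The color comes from a separate random roll, so it does not correspond to the power type.
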(event `self.ReceiveTick`
  (params (DeltaSeconds :type "Float (single-precision)"))
  (bind (_returnvalue_x _returnvalue_y) (`KismetMathLibrary.BreakVector` (* (* DeltaSeconds (`self.Var Speed`)) (`self.Var Direction`))))
  (`self.K2_AddActorWorldOffset` (`KismetMathLibrary.MakeVector` _returnvalue_x _returnvalue_y) true))

(fn `UserConstructionScript`
  (bind _returnvalue (`KismetMathLibrary.RandomIntegerInRange` 0 2))
  (bind _cone (`self.Cone`))
  (bind _output_get (set `self.power` (select `int` _returnvalue :`0` "NewEnumerator0" :`1` "NewEnumerator1" :`2` "NewEnumerator2" :!type "/Game/mystuff/blueprints/power-ups/e_powertype Enum")))
  ;[1 1 1] не понимаю почему цвета не подходят
  (switch `int` _returnvalue
    (:`0`
      (`PrimitiveComponent.SetMaterial` _cone 0 "/Game/mystuff/materials/mt_color_blue.mt_color_blue"))
    (:`1`
      (`PrimitiveComponent.SetMaterial` _cone 0 "/Game/mystuff/materials/mt_color_green.mt_color_green"))
    (:`2`
      (`PrimitiveComponent.SetMaterial` _cone 0 "/Game/mystuff/materials/mt_color_red.mt_color_red")))
  (`TextRenderComponent.K2_SetText` (`self.TextRender`) (`KismetTextLibrary.Conv_StringToText` (`|GetEnumeratorNameAsString` _output_get))))