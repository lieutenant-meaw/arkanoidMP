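; Grid spawner actor that creates the destructible blocks of a level and tracks when all of them are destroyed.
; The construction script previews the X-by-Y padded grid with static mesh components, which BeginPlay replaces with spawned Bp_block_Child actors.
; Each block's destroyed event adds its value to the pawn's score and increments a counter, firing the AllBlocksDestroyed dispatcher once it reaches the block total.
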(event `self.ReceiveBeginPlay`
  (bind (_returnvalue_x _returnvalue_y _returnvalue_z) (`KismetMathLibrary.BreakVector` (`self.K2_GetActorLocation`)))
  (bind _padding (`self.padding`))
  (`|ExecutionSequence`
    (:`then_0`
      ;[1 1 1] берем сначала павн
      (bind _returnvalue (`GameplayStatics.GetActorOfClass` "/Game/mystuff/blueprints/core/bp_pawn.bp_pawn_C"))
      (set `self.ourpawn` _returnvalue))
    (:`then_1`
      ;[1 1 1] удалить кубы для превью
      (for _array_element (`self.previewarray`)
        (`ActorComponent.K2_DestroyComponent` _array_element))
      (for _index (range (`self.x`))
        (for _index_2 (range (`self.y`))
          (bind _returnvalue_2 (`|SpawnActorFromClass` "/Game/mystuff/blueprints/bp_block_Child.bp_block_Child_C" (`KismetMathLibrary.MakeTransform` (`KismetMathLibrary.MakeVector` (+ (`KismetMathLibrary.Conv_IntToDouble` (* _index _padding)) _returnvalue_x) (+ _returnvalue_y (`KismetMathLibrary.Conv_IntToDouble` (* _index_2 _padding))) _returnvalue_z)) "Undefined" "OverrideRootScale" null null))
          (`KismetArrayLibrary.Array_Add` (`self.blocksarray`) _returnvalue_2)))
      (bind _blocknum (`self.blocks2win`))
      (set `self.BlockNum4Win` _blocknum)
      (for _array_element_2 (`self.blocksarray`)
        (add `/Game/mystuff/blueprints/bp_block.BlockDestroyed` _array_element_2 (delegate `BlockDestruction`))))))

(event `BlockDestruction`
  (params (Value :type Integer))
  (`/Game/mystuff/blueprints/core/bp_pawn.addedScore` (`self.ourpawn`) Value)
  ;[1 1 1] сравниваем количество мертвых блоков с количеством нужным для победы и вызываем ивент диспатчер
  (`/Engine/EditorBlueprintResources/StandardMacros.IncrementInt` (`self.deadblocks`)
    (:`  `
      (if (>= (`self.deadblocks`) (`self.BlockNum4Win`))
        (`self.allBlocksDestroyed`)))))

(fn `blocks2win`
  (returns (blocknum :type Integer))
  (return (`KismetArrayLibrary.Array_Length` (`self.blocksarray`))))

(fn `UserConstructionScript`
  (bind _padding (`self.padding`))
  ;[1 1 1] генерируем х на у кубов на выделенной площади с отступом в padding
  (for _index (range (`self.x`))
    (for _index_2 (range (`self.y`))
      (bind _returnvalue (`AddComponent|NODE_AddStaticMeshComponent-0` :`RelativeTransform` (`KismetMathLibrary.MakeTransform` (`KismetMathLibrary.MakeVector` (`KismetMathLibrary.Conv_IntToDouble` (* _index _padding)) (`KismetMathLibrary.Conv_IntToDouble` (* _index_2 _padding)) 50.0))))
      ;[1 1 1] пихаем эти кубы в массив на будущее
      (`KismetArrayLibrary.Array_Add` (`self.previewarray`) _returnvalue))))