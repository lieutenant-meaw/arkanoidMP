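; Player controller for a brick-breaker style game that drives the paddle pawn and manages the HUD and end screen.
; It caches the possessed bp_pawn, moves it sideways with a swept, frame-rate-scaled axis input and asks it to spawn a new ball on key press.
; The pawn's no-more-lives and the cube generator's all-blocks-destroyed dispatchers both trigger GameOver, which swaps the HUD for the win screen with UI-only input.
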(event `GameOver`
  ;[1 1 1] открываем меню для конца игры когда закончились блоки, event dispatcher "all blocks destroyed" находится в генераторе
  (set `Widget.Visibility` "Collapsed" (`self.HUD`))
  (bind _returnvalue (`|CreateWidget` "/Game/mystuff/ui/wbp_winscreen.wbp_winscreen_C" self))
  (`UserWidget.AddToViewport` _returnvalue 0)
  (`WidgetBlueprintLibrary.SetInputMode_UIOnlyEx` self _returnvalue)
  (set `self.bShowMouseCursor` true))

(event `self.ReceiveBeginPlay`
  (`|ExecutionSequence`
    (:`then_0`
      ;[1 1 1] ключаем HUD сразу как игра начинается
      (`WidgetBlueprintLibrary.SetInputMode_GameOnly` self)
      (bind _returnvalue (`|CreateWidget` "/Game/mystuff/ui/wbp_HUD.wbp_HUD_C" self))
      (bind _output_get (set `self.HUD` _returnvalue))
      (`UserWidget.AddToViewport` _output_get 0))
    (:`then_1`
      ;[1 1 1] открываем меню для конца игры когда закончились блоки, event dispatcher "all blocks destroyed" находится в генераторе
      (bind _returnvalue_2 (`GameplayStatics.GetActorOfClass` "/Game/mystuff/blueprints/bp_cubesgenerator.bp_cubesgenerator_C"))
      (add `/Game/mystuff/blueprints/bp_cubesgenerator.allBlocksDestroyed` _returnvalue_2 (delegate `GameOver`)))))

(event `self.ReceivePossess`
  (params (PossessedPawn :type "Pawn Object Reference"))
  ;[1 1 1] подключаем управление
  (bind _asbp_pawn (cast `/Game/mystuff/blueprints/core/bp_pawn` PossessedPawn))
  (bind _output_get (set `self.MyPawn` _asbp_pawn))
  ;[1 1 1] открываем меню для конца игры когда закончились блоки, event dispatcher "all blocks destroyed" находится в генераторе
  (add `/Game/mystuff/blueprints/core/bp_pawn.noMoreLives` _output_get (delegate `GameOver`)))

(event `InputAxis|left-right`
  (params (AxisValue :type "Float (single-precision)"))
  ;[1 1 1] влево-вправо
  (`self.K2_AddActorWorldOffset` (`self.MyPawn`) (`KismetMathLibrary.MakeVector` 0.0 (* AxisValue (`GameplayStatics.GetWorldDeltaSeconds`) (`self.speed`))) true false))

(event `InputAction|respawn the ball`
  (params (Key :type "Key Structure"))
  ;[1 1 1] новый мячик
  (:`Pressed`
    (`/Game/mystuff/blueprints/core/bp_pawn.spawnball` (`self.MyPawn`))))

(fn `UserConstructionScript`)