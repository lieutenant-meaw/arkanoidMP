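; Player pawn for a ball game with lives, score and power-ups, built around a scalable Cube and an Arrow spawn point.
; Spawning a ball costs a life and only happens when none exists, signalling when lives run out.
; Overlapped power-ups add score, then grant a life, extra balls or a wider Cube before being destroyed.
; Widening stacks, and a retriggerable delay restores the starting scale after the last pickup.
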(event `spawnball`
  ;[1 1 1] по нажатию кнопки спавним мячик, если его нет
  (`self.existingball`
    (:`then`)
    (:`else`
      (bind _result (`/Engine/EditorBlueprintResources/StandardMacros.DecrementInt` (`self.lives`))
        (:`  `
          (bind _output_get (set `self.lives` _result))
          (`self.LivesChange` _output_get)
          (if (>= _output_get 0)
            (`SceneComponent.SetVisibility` (`self.howtotext`) true false)
            (bind _returnvalue (`|SpawnActorFromClass` "/Game/mystuff/blueprints/bp_ball.bp_ball_C" (`KismetMathLibrary.MakeTransform` (`SceneComponent.K2_GetComponentLocation` (`self.Arrow`)) (struct) (0.7 0.7 0.7)) "AdjustIfPossibleButAlwaysSpawn" "OverrideRootScale" null null))
            (set `self.existingball` _returnvalue)
            (`SceneComponent.SetVisibility` (`self.howtotext`) false false)
            (else
              (`self.noMoreLives`))))))))

(event `self.Cube.OnComponentBeginOverlap`
  (params (OverlappedComponent :type "PrimitiveComponent Object Reference") (OtherActor :type "Actor Object Reference") (OtherComp :type "PrimitiveComponent Object Reference") (OtherBodyIndex :type Integer) (bFromSweep :type Boolean) (SweepResult :type "HitResult Structure (by ref)"))
  ;[1 1 1] тригерим power up при касании, и потом ломаем
  (bind _asbp_power_base (cast `/Game/mystuff/blueprints/power-ups/bp_power_base` OtherActor))
  (switch `/Game/mystuff/blueprints/power-ups/e_powertype` (`/Game/mystuff/blueprints/power-ups/bp_power_base.power` _asbp_power_base)
    (:`NewEnumerator0`
      (`self.hugeEvent`))
    (:`NewEnumerator1`
      (`self.lifeEvent`))
    (:`NewEnumerator2`
      (`self.ballsEvent`)))
  (`self.addedScore` 50)
  (`self.K2_DestroyActor` OtherActor))

(event `lifeEvent`
  ;[1 1 1] бонусная жизнь
  (bind _result (`/Engine/EditorBlueprintResources/StandardMacros.IncrementInt` (`self.lives`))
    (:`  `
      (`self.LivesChange` _result)
      (`KismetSystemLibrary.PrintString` "+1 life"))))

(event `ballsEvent`
  (bind (_returnvalue_x _returnvalue_y _returnvalue_z) (`KismetMathLibrary.BreakVector` (`SceneComponent.K2_GetComponentLocation` (`self.Arrow`))))
  ;[1 1 1] спавним еще мячиков
  (for _index (range 4)
    (`|SpawnActorFromClass` "/Game/mystuff/blueprints/bp_ball.bp_ball_C" (`KismetMathLibrary.MakeTransform` (`KismetMathLibrary.MakeVector` _returnvalue_x (+ (* _index 51) _returnvalue_y) _returnvalue_z) (struct) (0.5 0.5 0.5)) "AdjustIfPossibleButDontSpawnIfColliding" "OverrideRootScale" null null)
    (`KismetSystemLibrary.PrintString` "balls")))

(event `hugeEvent`
  (bind _cube (`self.Cube`))
  (bind (_relativescale3d_x _relativescale3d_y _relativescale3d_z) (`KismetMathLibrary.BreakVector` (`SceneComponent.RelativeScale3D` _cube)))
  ;[1 1 1] увеличиваем размер
  (`SceneComponent.SetRelativeScale3D` _cube (`KismetMathLibrary.MakeVector` _relativescale3d_x (* _relativescale3d_y 1.5) _relativescale3d_z))
  (`self.minimizeEvent`)
  (`KismetSystemLibrary.PrintString` "+size"))

(event `self.ReceiveBeginPlay`
  ;[1 1 1] сохраняем стартовый размер
  (set `self.startscale` (`SceneComponent.RelativeScale3D` (`self.Cube`))))

(event `minimizeEvent`
  ;[1 1 1] возвращаем старый размер. этот delay обнуляет таймер если его тригерят снова, поэтому бонус можно накапливать если получить его несколько раз, он будет обнулять таймер каждый раз, стакая бонус каждый раз
  (`KismetSystemLibrary.RetriggerableDelay` 3.0)
  (`SceneComponent.SetRelativeScale3D` (`self.Cube`) (`self.startscale`))
  (`KismetSystemLibrary.PrintString` "back to normal"))

(fn `addedScore`
  (params (value :type Integer))
  ;[1 1 1] на всякий случай прибавляем абсолютное значение в total score. Делаем это через функцию ибо
  (bind _output_get (set `self.totalScore` (+ (`KismetMathLibrary.Abs_Int` value) (`self.totalScore`))))
  (`self.ScoreChange` _output_get))

(fn `UserConstructionScript`)