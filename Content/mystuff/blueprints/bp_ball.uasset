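; Ball actor that travels on the XY plane and bounces off whatever blocks it.
; Tick applies a frame-rate-independent, swept world offset from its direction and speed.
; A blocking hit reflects the direction around the hit normal and adds a speed increment, capped by Min.
; An author comment reports an unresolved bug where speed drops instead of rising.
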(event `self.ReceiveTick`
  (params (DeltaSeconds :type "Float (single-precision)"))
  (bind (_returnvalue_x _returnvalue_y) (`KismetMathLibrary.BreakVector` (* (* DeltaSeconds (`self.var_speed`)) (`self.var_direction`))))
  ;[1 1 1] каждый кадр, умножая скорость на время между кадрами (чтобы вне зависимости от фпс скорость была одна) двигаем актёра в выбранном направлении
  (bind _sweephitresult (`self.K2_AddActorWorldOffset` (`KismetMathLibrary.MakeVector` _returnvalue_x _returnvalue_y) true))
  (bind (_bblockinghit _binitialoverlap _time _distance _location _impactpoint _normal) (`GameplayStatics.BreakHitResult` _sweephitresult))
  ;[1 1 1] если ударил что нюдь
  (if _bblockinghit
    ;[1 1 1] отразил
    (set `self.var_direction` (`KismetMathLibrary.GetReflectionVector` (`self.var_direction`) _normal))
    ;[1 1 1] увеличиваем скорость после каждого столкновения
    (bind _output_get (set `self.var_speed` (`KismetMathLibrary.FMin` 2000.0 (+ (`self.var_speed`) (`self.var_deltaspeed`)))))))

(fn `UserConstructionScript`)