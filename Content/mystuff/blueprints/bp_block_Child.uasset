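; Child block Blueprint that drops a power actor when destroyed, if it is a gold block.
; On BeginPlay it checks whether the cube's first material is the gold metal one and, only then, binds to its own OnDestroyed event.
; That handler always spawns a Bp_power_base at the block's location with a fixed rotation, regardless of collision.
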(event `self.ReceiveBeginPlay`
  (if (== (`PrimitiveComponent.GetMaterial` (`self.Cube`) 0) "/Game/mystuff/materials/metal/mt_metal_gold.mt_metal_gold")
    (add `self.OnDestroyed` (delegate `spawnpower`))))

(event `spawnpower` :!signature `self.OnDestroyed`
  (params (DestroyedActor :type "Actor Object Reference"))
  (`|SpawnActorFromClass` "/Game/mystuff/blueprints/power-ups/bp_power_base.bp_power_base_C" (`KismetMathLibrary.MakeTransform` (`self.K2_GetActorLocation`) (struct :`Pitch` -90.0)) "AlwaysSpawn" "OverrideRootScale" null null))

(fn `UserConstructionScript`
  (`parent.UserConstructionScript`))